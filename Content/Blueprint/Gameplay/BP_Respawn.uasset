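; BP_Respawn is a trigger volume that sends the BP_FirstPerson character back to a spawn point.
; Overlapping its box starts a quick camera fade-out, then after a short delay stops the character's movement and teleports it to the SpawnPoint actor's location with zeroed rotation.
; Another brief delay precedes a camera fade back in, so the relocation happens behind the fade.
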(event `self.Box.OnComponentBeginOverlap`
  (params (OverlappedComponent :type "PrimitiveComponent Object Reference") (OtherActor :type "Actor Object Reference") (OtherComp :type "PrimitiveComponent Object Reference") (OtherBodyIndex :type Integer) (bFromSweep :type Boolean) (SweepResult :type "HitResult Structure (by ref)"))
  (bind _asbp_first_person (cast `/Game/Blueprint/Characters/BP_FirstPerson` OtherActor))
  (`|ExecutionSequence`
    (:`then_0`
      (`PlayerCameraManager.StartCameraFade` :`self` (`GameplayStatics.GetPlayerCameraManager` 0) :`ToAlpha` 1.0 :`Duration` 0.2 :`bHoldWhenFinished` true))
    (:`then_1`
      (`KismetSystemLibrary.Delay` 0.2)
      (`MovementComponent.StopMovementImmediately` (`Character.CharacterMovement` _asbp_first_person))
      (`self.K2_TeleportTo` :`self` _asbp_first_person :`DestLocation` (`self.K2_GetActorLocation` (`self.SpawnPoint`)))
      (`KismetSystemLibrary.Delay` 0.1)
      (`PlayerCameraManager.StartCameraFade` :`self` (`GameplayStatics.GetPlayerCameraManager` 0) :`FromAlpha` 0.1 :`Duration` 0.5 :`bHoldWhenFinished` true))))

(fn `UserConstructionScript`)