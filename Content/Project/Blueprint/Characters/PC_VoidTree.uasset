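; PC_VoidTree is the player controller that sets up first-person input for the player.
; On possess it adds the IMC_VoidTree Enhanced Input mapping context, and on begin play it switches to game-only input with the cursor hidden.
; Look input drives yaw and pitch, with pitch sign chosen by an InvertCamera flag.
; Sprint input swaps the controlled BP_FirstPerson's max walk speed between that pawn's sprint and walk values.
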(event `self.ReceivePossess`
  (params (PossessedPawn :type "Pawn Object Reference"))
  (`EnhancedInputSubsystemInterface.AddMappingContext` (subsystem `EnhancedInputLocalPlayerSubsystem`) "/Game/Project/Input/IMC_VoidTree.IMC_VoidTree" 0 (struct)))

(event `self.ReceiveBeginPlay`
  (`WidgetBlueprintLibrary.SetInputMode_GameOnly` (`GameplayStatics.GetPlayerController` 0))
  (set `self.bShowMouseCursor` false))

(event `EnhancedInput|/Game/Project/Input/IA_Look`
  (params (ActionValue :type "Vector2D Structure") (ElapsedSeconds :type "Float (double-precision)") (TriggeredSeconds :type "Float (double-precision)") (InputAction :type "InputAction Object Reference" :default "/Game/Project/Input/IA_Look.IA_Look"))
  (bind (_x _y) (`KismetMathLibrary.BreakVector2D` ActionValue))
  ; Camera
  (:`Triggered`
    (`self.AddYawInput` _x) ; Turn
    (`self.AddPitchInput` (* _y (`KismetMathLibrary.SelectFloat` 1.0 -1.0 (`self.InvertCamera`)))) ; Look
  ))

(event `EnhancedInput|/Game/Project/Input/IA_Sprint`
  (params (ActionValue :type "Vector2D Structure") (ElapsedSeconds :type "Float (double-precision)") (TriggeredSeconds :type "Float (double-precision)") (InputAction :type "InputAction Object Reference" :default "/Game/Project/Input/IA_Sprint.IA_Sprint"))
  ; Sprint
  (:`Started`
    (bind _asbp_first_person (cast `/Game/Project/Blueprint/Characters/BP_FirstPerson` (`self.K2_GetPawn`)))
    (set `CharacterMovementComponent.MaxWalkSpeed` (`/Game/Project/Blueprint/Characters/BP_FirstPerson.Sprint Speed` _asbp_first_person) (`Character.CharacterMovement` _asbp_first_person)))
  (:`Completed`
    (bind _asbp_first_person_2 (cast `/Game/Project/Blueprint/Characters/BP_FirstPerson` (`self.K2_GetPawn`)))
    (set `CharacterMovementComponent.MaxWalkSpeed` (`/Game/Project/Blueprint/Characters/BP_FirstPerson.Walk Speed` _asbp_first_person_2) (`Character.CharacterMovement` _asbp_first_person_2))))

(fn `UserConstructionScript`)