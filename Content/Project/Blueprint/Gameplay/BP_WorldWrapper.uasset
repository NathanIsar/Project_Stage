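; BP_WorldWrapper wraps the first-person player vertically, creating a looping world of height LengthTree.
; Overlapping BasBox teleports the character up by that length and HautBox teleports it down, each adjusted by OffsetTree, with rotation zeroed.
; Each jump is masked by briefly hiding the character, resetting temporal AA, disabling motion blur and flagging a camera cut, while LaunchCharacter reapplies its velocity.
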(event `self.BasBox.OnComponentBeginOverlap`
  (params (OverlappedComponent :type "PrimitiveComponent Object Reference") (OtherActor :type "Actor Object Reference") (OtherComp :type "PrimitiveComponent Object Reference") (OtherBodyIndex :type Integer) (bFromSweep :type Boolean) (SweepResult :type "HitResult Structure (by ref)"))
  (bind _asbp_first_person (cast `/Game/Project/Blueprint/Characters/BP_FirstPerson` OtherActor))
  (`KismetSystemLibrary.ExecuteConsoleCommand` "r.TemporalAA.Reset 1" null)
  (`KismetSystemLibrary.ExecuteConsoleCommand` "r.MotionBlur.Amount 0" null)
  (`self.SetActorHiddenInGame` _asbp_first_person true)
  (`self.K2_TeleportTo` :`self` _asbp_first_person :`DestLocation` (`KismetMathLibrary.MakeVector` (.x (`self.K2_GetActorLocation` _asbp_first_person)) (.y (`self.K2_GetActorLocation` _asbp_first_person)) (- (+ (.z (`self.K2_GetActorLocation` _asbp_first_person)) (`self.LengthTree`)) (`self.OffsetTree`))))
  (`PlayerCameraManager.SetGameCameraCutThisFrame` (`GameplayStatics.GetPlayerCameraManager` 0))
  (`Character.LaunchCharacter` _asbp_first_person (`self.GetVelocity` _asbp_first_person) true true)
  (`KismetSystemLibrary.Delay` 0.05)
  (`self.SetActorHiddenInGame` _asbp_first_person false)
  (`KismetSystemLibrary.Delay` 0.0)
  (`KismetSystemLibrary.ExecuteConsoleCommand` "r.MotionBlur.Amount 1" null))

(event `self.HautBox.OnComponentBeginOverlap`
  (params (OverlappedComponent :type "PrimitiveComponent Object Reference") (OtherActor :type "Actor Object Reference") (OtherComp :type "PrimitiveComponent Object Reference") (OtherBodyIndex :type Integer) (bFromSweep :type Boolean) (SweepResult :type "HitResult Structure (by ref)"))
  (bind _asbp_first_person (cast `/Game/Project/Blueprint/Characters/BP_FirstPerson` OtherActor))
  (`KismetSystemLibrary.ExecuteConsoleCommand` "r.TemporalAA.Reset 1" null)
  (`KismetSystemLibrary.ExecuteConsoleCommand` "r.MotionBlur.Amount 0" null)
  (`self.SetActorHiddenInGame` _asbp_first_person true)
  (`self.K2_TeleportTo` :`self` _asbp_first_person :`DestLocation` (`KismetMathLibrary.MakeVector` (.x (`self.K2_GetActorLocation` _asbp_first_person)) (.y (`self.K2_GetActorLocation` _asbp_first_person)) (+ (- (.z (`self.K2_GetActorLocation` _asbp_first_person)) (`self.LengthTree`)) (`self.OffsetTree`))))
  (`PlayerCameraManager.SetGameCameraCutThisFrame` (`GameplayStatics.GetPlayerCameraManager` 0))
  (`Character.LaunchCharacter` _asbp_first_person (`self.GetVelocity` _asbp_first_person) true true)
  (`KismetSystemLibrary.Delay` 0.05)
  (`self.SetActorHiddenInGame` _asbp_first_person false)
  (`KismetSystemLibrary.Delay` 0.0)
  (`KismetSystemLibrary.ExecuteConsoleCommand` "r.MotionBlur.Amount 1" null))

(fn `UserConstructionScript`)